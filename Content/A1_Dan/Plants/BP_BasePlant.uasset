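; Base plant that shrimp characters harvest to add to their hunger value, drawing on a limited food supply.
; A range overlap registers the plant with shrimp while food remains, and Harvested feeds the harvester and deducts one serving.
; When too little food remains, it unregisters from all tracked shrimp and hides its mesh through a rep-prefixed event.
; An empty harvest animation event fires on each harvest as a hook.
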(event OnComponentBeginOverlap(HarvestRange)
  (params (OverlappedComponent :type Primitive%20Component%20Object%20Reference) (OtherActor :type Actor%20Object%20Reference) (OtherComp :type Primitive%20Component%20Object%20Reference) (OtherBodyIndex :type Integer) (bFromSweep :type Boolean) (SweepResult :type Hit%20Result%20Structure%20%28by%20ref%29))
  (bind _asbp_shrimp_character (Utilities|Casting|CastToBP_ShrimpCharacter OtherActor))
  (bind _can_be_havested (CallFunction|CanbeHarvested))
  (if _can_be_havested
    (CallFunction|ShrimpinRange _asbp_shrimp_character)))

(event OnComponentEndOverlap(HarvestRange)
  (params (OverlappedComponent :type Primitive%20Component%20Object%20Reference) (OtherActor :type Actor%20Object%20Reference) (OtherComp :type Primitive%20Component%20Object%20Reference) (OtherBodyIndex :type Integer))
  (bind _asbp_shrimp_character (Utilities|Casting|CastToBP_ShrimpCharacter OtherActor))
  (CallFunction|ShrimpOutOfRange _asbp_shrimp_character))

(event Custom|repFoodDepleted
  (CallFunction|FoodDepleted))

(event Custom|repHarvestAnimHook)

(event EventBeginPlay
  (CallFunction|InitPlant))

(fn ConstructionScript)

(fn Harvested
  (params (harvester :type BP%20Shrimp%20Character%20Object%20Reference))
  (bind _can_be_havested (CallFunction|CanbeHarvested))
  (if _can_be_havested
    (Default|RepAddHunger harvester (Variables|Default|GetfoodValue))
    (CallFunction|DeductFoodValue)
    (CallFunction|RepHarvestAnimHook)))

(fn CanbeHarvested
  (return (>= (Variables|Default|GetavailableFood) (Variables|Default|GetfoodValue))))

(fn ShrimpinRange
  (params (shrimp :type BP%20Shrimp%20Character%20Object%20Reference))
  (Default|AddPlantinRange shrimp self)
  (Utilities|Array|Add (Variables|Default|GetinteractingShrimps) shrimp))

(fn ShrimpOutOfRange
  (params (shrimp :type BP%20Shrimp%20Character%20Object%20Reference))
  (Default|RemovePlantinRange shrimp self)
  (Utilities|Array|RemoveItem (Variables|Default|GetinteractingShrimps) shrimp))

(fn InitPlant
  (Variables|Default|SetavailableFood (Variables|Default|GetmaxAvailableFood)))

(fn DeductFoodValue
  (bind _output_get (Variables|Default|SetavailableFood (- (Variables|Default|GetavailableFood) (Variables|Default|GetfoodValue))))
  (if (< _output_get (Variables|Default|GetfoodValue))
    (CallFunction|RepFoodDepleted)
    (for _array_element (Variables|Default|GetinteractingShrimps)
      (Default|RemovePlantinRange _array_element self))
    (Utilities|Array|Clear (Variables|Default|GetinteractingShrimps))))

(fn FoodDepleted
  (Rendering|SetVisibility (Variables|Default|GetSkeletalMesh) false true))