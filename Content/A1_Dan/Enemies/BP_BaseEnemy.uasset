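; BP_BaseEnemy is a base enemy that swims idly until it spots the shrimp player character, then pursues it.
; PawnSensing stores the seen shrimp as Target, and Tick moves straight toward it at Speed, or calls SwimInLoop to drift forward and rightward without one.
; Overlapping the InRange component halts movement and fires RepAttack, an empty event here, while leaving range resumes the chase.
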(event OnSeePawn(PawnSensing)
  (params (Pawn :type Pawn%20Object%20Reference))
  (bind _asbp_shrimp_character (Utilities|Casting|CastToBP_ShrimpCharacter Pawn))
  (Variables|Default|Settarget _asbp_shrimp_character))

(event OnComponentBeginOverlap(inRange)
  (params (OverlappedComponent :type Primitive%20Component%20Object%20Reference) (OtherActor :type Actor%20Object%20Reference) (OtherComp :type Primitive%20Component%20Object%20Reference) (OtherBodyIndex :type Integer) (bFromSweep :type Boolean) (SweepResult :type Hit%20Result%20Structure%20%28by%20ref%29))
  (if (== OtherActor (Variables|Default|Gettarget))
    (Variables|Default|SettargetReached true)
    (Components|Movement|StopMovementImmediately (Variables|Character|GetCharacterMovement))
    (CallFunction|RepAttack)))

(event OnComponentEndOverlap(inRange)
  (params (OverlappedComponent :type Primitive%20Component%20Object%20Reference) (OtherActor :type Actor%20Object%20Reference) (OtherComp :type Primitive%20Component%20Object%20Reference) (OtherBodyIndex :type Integer))
  (if (== OtherActor (Variables|Default|Gettarget))
    (Variables|Default|SettargetReached false)))

(event Custom|repAttack)

(event EventTick
  (params (DeltaSeconds :type Float%20%28single-precision%29))
  (Utilities|IsValid (Variables|Default|Gettarget)
    (:Is%20Valid
      (if (not (Variables|Default|GettargetReached))
        (Pawn|Input|AddMovementInput (Math|Vector|GetUnitDirection(Vector) (Transformation|GetActorLocation) (Transformation|GetActorLocation (Variables|Default|Gettarget))) (Variables|Default|Getspeed) false)))
    (:Is%20Not%20Valid
      (CallFunction|SwiminLoop))))

(fn ConstructionScript)

(fn SwiminLoop
  (Pawn|Input|AddMovementInput (+ (Transformation|GetActorForwardVector) (/ (Transformation|GetActorRightVector) (Variables|Default|GetpassiveLoopSizeModifier))) 1.0 false))