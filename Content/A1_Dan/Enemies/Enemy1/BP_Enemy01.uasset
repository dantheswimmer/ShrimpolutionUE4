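; Enemy 01 Blueprint for an enemy that attacks with a bite and damages its target.
; On BeginPlay it caches its Enemy01AnimBP instance and hands it a reference back to itself.
; RepAttack sets the bite flag on that AnimBP, while a separate damageTarget event applies fixed damage through the target's RepTakeDamage.
; An unconnected node for snapping the target to the Mouth never runs.
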(event Custom|damageTarget
  (Default|RepTakeDamage (Variables|Default|Gettarget) 200))

(event EventBeginPlay
  (CallFunction|InitAnim))

(event Collision|EventActorBeginOverlap
  (params (OtherActor :type Actor%20Object%20Reference)))

(event EventTick
  (params (DeltaSeconds :type Float%20%28single-precision%29)))

(event EventRepAttack
  (Variables|/Game/A1_Dan/Enemies/Enemy1/Enemy01AnimBP.Enemy01AnimBP_C|SetabpBite (Variables|Default|Getanimbp) true))

(fn ConstructionScript
  (|CallParentFunction))

(fn InitAnim
  (bind _asenemy_01anim_bp (Utilities|Casting|CastToEnemy01AnimBP (Components|SkeletalMesh|GetAnimInstance (Variables|Character|GetMesh))))
  (Variables|/Game/A1_Dan/Enemies/Enemy1/Enemy01AnimBP.Enemy01AnimBP_C|SetowningEnemy _asenemy_01anim_bp self)
  (Variables|Default|Setanimbp _asenemy_01anim_bp))