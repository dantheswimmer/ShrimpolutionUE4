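; BP_ShrimpHUD is a HUD Blueprint that shows and hides the matchmaking main menu.
; DisplayMatchmakingMenu lazily creates and caches the widget for player controller 0, then makes it visible; RemoveMatchmakingMenu hides it rather than destroying it.
; Helper functions switch between UI-only input with a visible cursor and game-only input without one.
; The event graph is empty, so other code must call these functions.
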(event EventBeginPlay)

(event Collision|EventActorBeginOverlap
  (params (OtherActor :type Actor%20Object%20Reference)))

(event EventTick
  (params (DeltaSeconds :type Float%20%28single-precision%29)))

(fn ConstructionScript)

(fn DisplayMatchmakingMenu
  (Utilities|IsValid (Variables|Default|GetmatchmakingMenu)
    (:Is%20Valid
      _)
    (:Is%20Not%20Valid
      (bind _returnvalue (UserInterface|CreateWidget "/Game/A1_Dan/MatchMaking/matchmakingMainMenu.matchmakingMainMenu_C" (Game|GetPlayerController 0)))
      (bind _output_get (Variables|Default|SetmatchmakingMenu _returnvalue))
      (UserInterface|Viewport|AddtoViewport (Variables|Default|GetmatchmakingMenu) 0)))
  (Widget|SetVisibility (Variables|Default|GetmatchmakingMenu) "Visible")
  (CallFunction|EnterUIMode _output_get))

(fn RemoveMatchmakingMenu
  (Widget|SetVisibility (Variables|Default|GetmatchmakingMenu) "Hidden")
  (CallFunction|ExitUIMode))

(fn EnterUIMode
  (params (widget%20to%20focus :type Widget%20Object%20Reference))
  (bind _returnvalue (Game|GetPlayerController 0))
  (Input|SetInputModeUIOnly _returnvalue widget%20to%20focus "DoNotLock")
  (Variables|/Script/Engine.PlayerController|SetbShowMouseCursor _returnvalue true))

(fn ExitUIMode
  (bind _returnvalue (Game|GetPlayerController 0))
  (Input|SetInputModeGameOnly _returnvalue)
  (Variables|/Script/Engine.PlayerController|SetbShowMouseCursor _returnvalue false))